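; Player character Blueprint with directional movement, sprinting, a low-gravity hover and basic health.
; Holding Jump jumps and sets a hover flag, which Tick reads to lower gravity scale until release.
; Run swaps walk and sprint speeds, while jumping, sprinting and landing spawn shockwave effects, the latter two at a fixed world Z.
; Damage reduces clamped health and calls an empty Died event at zero.
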(event Custom|Died)

(event EventTick
  (params (DeltaSeconds :type Float%20%28single-precision%29))
  (bind _charactermovement (Variables|Character|GetCharacterMovement))
  (Utilities|FlowControl|Sequence
    (:then_0
      (if (Variables|Default|GetIsHovering)
        (Variables|/Script/Engine.CharacterMovementComponent|SetGravityScale _charactermovement 0.2)
        (else
          (Variables|/Script/Engine.CharacterMovementComponent|SetGravityScale _charactermovement 1.0))))))

(event EventOnLanded
  (params (Hit :type Hit%20Result%20Structure%20%28by%20ref%29))
  (bind _returnvalue (Transformation|GetActorLocation))
  (Niagara|SpawnSystematLocation "/Game/Vefects/Easy_Shockwaves_VFX/VFX/Shockwaves/Particles/Color_Variation/VFX_Shockwave_01_Lavender_Big_1s.VFX_Shockwave_01_Lavender_Big_1s" (Math|Vector|MakeVector (.x _returnvalue) (.y _returnvalue) -7e+01)))

(event EventBeginPlay
  (Variables|Default|SetHealth (Variables|Default|GetMax%20Health)))

(event Game|Damage|EventAnyDamage
  (params (Damage :type Float%20%28single-precision%29) (DamageType :type Damage%20Type%20Object%20Reference) (InstigatedBy :type Controller%20Object%20Reference) (DamageCauser :type Actor%20Object%20Reference))
  (Variables|Default|SetHealth (Math|Float|Clamp(Float) (- (Variables|Default|GetHealth) Damage) 0.0 (Variables|Default|GetMax%20Health)))
  (if (<= (Variables|Default|GetHealth) 0.0)
    (CallFunction|Died)))

(event Input|ActionEvents|InputActionJump
  (params (Key :type Key%20Structure :default "None"))
  (:Pressed
    (Variables|Default|SetIsHovering true)
    (Character|Jump)
    (Niagara|SpawnSystematLocation "/Game/Vefects/Easy_Shockwaves_VFX/VFX/Shockwaves/Particles/Color_Variation/VFX_Shockwave_01_Lavender_Big_1s.VFX_Shockwave_01_Lavender_Big_1s" (Transformation|GetActorLocation)))
  (:Released
    (Variables|Default|SetIsHovering false)
    (Character|StopJumping)))

(event Input|ActionEvents|InputActionRun
  (params (Key :type Key%20Structure :default "None"))
  (bind _returnvalue (Transformation|GetActorLocation))
  (bind _charactermovement (Variables|Character|GetCharacterMovement))
  (:Pressed
    (Variables|/Script/Engine.CharacterMovementComponent|SetMaxWalkSpeed _charactermovement (Variables|Default|GetSpring%20Speed))
    (Variables|Default|SetIsSprinting true)
    (Niagara|SpawnSystematLocation "/Game/Vefects/Easy_Shockwaves_VFX/VFX/Shockwaves/Particles/Vertical/VFX_Shockwave_Vertical_02_White_Big_1s.VFX_Shockwave_Vertical_02_White_Big_1s" (Math|Vector|MakeVector (.x _returnvalue) (.y _returnvalue) -7e+01)))
  (:Released
    (Variables|/Script/Engine.CharacterMovementComponent|SetMaxWalkSpeed _charactermovement (Variables|Default|GetWalk%20Speed))
    (Variables|Default|SetIsSprinting false)))

(event Input|AxisEvents|InputAxisMoveForward
  (params (AxisValue :type Float%20%28single-precision%29))
  (Pawn|Input|AddMovementInput (Transformation|GetActorForwardVector) AxisValue false))

(event Input|AxisEvents|InputAxisMoveRight
  (params (AxisValue :type Float%20%28single-precision%29))
  (Pawn|Input|AddMovementInput (Transformation|GetActorRightVector) AxisValue false))

(fn ConstructionScript)